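; BP_Socket is a named spawn socket that launches turtle actors toward a linked finish point.
; BeginPlay shows the socket's name on its text component.
; SpawnTurtle spawns a scaled-down BP_Turtle at the spawn point and, if the finish point is valid, passes it the finish point, movement method and socket before calling ReadyToWork.
; It also spawns a lightning effect with sound as the spawn animation.
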(event `self.ReceiveBeginPlay`
  (`TextRenderComponent.K2_SetText` (`self.SocketNameText`) (`KismetTextLibrary.Conv_NameToText` (`self.Name`))))

(fn `SpawnTurtle`
  (bind _finishpoint (`self.FinishPoint`))
  (bind _returnvalue (`SceneComponent.K2_GetComponentLocation` (`self.SpawnPoint`)))
  ;[1 1 1] Спавн "черепашки"
  (bind _returnvalue_2 (`|SpawnActorFromClass` "/Game/Blueprints/BP_Turtle.BP_Turtle_C" (`KismetMathLibrary.MakeTransform` _returnvalue (struct) (0.7 0.7 0.7)) "Undefined" "OverrideRootScale" null null null))
  (`|ExecutionSequence`
    (:`then_0`
      (`/Engine/EditorBlueprintResources/StandardMacros.IsValid` _finishpoint
        (:`Is Valid`
          ;[1 1 1] Установка значений для "черепашки", вызов события
          (set `/Game/Blueprints/BP_Turtle.FinishPoint` _finishpoint _returnvalue_2)
          (set `/Game/Blueprints/BP_Turtle.NumberOfTurtle` (`self.MoveMethod`) _returnvalue_2)
          (set `/Game/Blueprints/BP_Turtle.StartPosition` self _returnvalue_2)
          (`/Game/Blueprints/BP_Turtle.ReadyToWork` _returnvalue_2))))
    (:`then_1`
      ;[1 1 1] Анимация спавна "черепашки"
      (`|SpawnActorFromClass` "/Game/FXVarietyPack/Blueprints/BP_ky_lightning3.BP_ky_lightning3_C" (`KismetMathLibrary.MakeTransform` (`KismetMathLibrary.MakeVector` (.x _returnvalue) (.y _returnvalue) 130.0)) "AlwaysSpawn" "OverrideRootScale" null "/Game/Sound/SLighting.SLighting" null))))

(fn `UserConstructionScript`)