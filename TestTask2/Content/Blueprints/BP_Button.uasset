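; BP_Button is an interactable button that spawns a turtle through its linked Socket (nest) when pressed.
; EnterTrigger overlaps show or hide the ThirdPersonCharacter's InteractIcon.
; Interact prints a debug message, rewinds the Click timeline and fires OnInteract.
; OnInteract plays Click to lerp the Button's relative location for the press animation, then calls SpawnTurtle on the Socket if it is valid.
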(event `self.EnterTrigger.OnComponentBeginOverlap`
  (params (OverlappedComponent :type "PrimitiveComponent Object Reference") (OtherActor :type "Actor Object Reference") (OtherComp :type "PrimitiveComponent Object Reference") (OtherBodyIndex :type Integer) (bFromSweep :type Boolean) (SweepResult :type "HitResult Structure (by ref)"))
  ;[1 1 1] Для показа таблички о взаимодействии
  (bind _asthird_person_character (cast `/Game/ThirdPersonBP/Blueprints/ThirdPersonCharacter` OtherActor))
  (`Widget.SetVisibility` (`/Game/ThirdPersonBP/Blueprints/ThirdPersonCharacter.InteractIcon` _asthird_person_character) "Visible"))

(event `self.EnterTrigger.OnComponentEndOverlap`
  (params (OverlappedComponent :type "PrimitiveComponent Object Reference") (OtherActor :type "Actor Object Reference") (OtherComp :type "PrimitiveComponent Object Reference") (OtherBodyIndex :type Integer))
  ;[1 1 1] Для скрытия таблички о взаимодействии
  (bind _asthird_person_character (cast `/Game/ThirdPersonBP/Blueprints/ThirdPersonCharacter` OtherActor))
  (`Widget.SetVisibility` (`/Game/ThirdPersonBP/Blueprints/ThirdPersonCharacter.InteractIcon` _asthird_person_character) "Hidden"))

(event `On Interact`
  (bind _socket (`self.Socket`))
  (`|ExecutionSequence`
    (:`then_0`
      ;[1 1 1] Анимация нажатия кнопки
      (bind (_direction _float) (`Timeline|Click`)
        (:`Update`
          (`SceneComponent.K2_SetRelativeLocation` (`self.Button`) (`KismetMathLibrary.VLerp` (0.0 0.0 150.0) (0.0 -10.0 150.0) _float) false false))))
    (:`then_1`
      ;[1 1 1] Спавн "черепашки", вызывает функцию гнезда
      (`/Engine/EditorBlueprintResources/StandardMacros.IsValid` _socket
        (:`Is Valid`
          (`/Game/Blueprints/BP_Socket.SpawnTurtle` _socket))))))

(fn `Interact`
  (returns (Success :type Boolean))
  (`KismetSystemLibrary.PrintString` (`KismetStringLibrary.Concat_StrStr` "Нажата кнопка " (`KismetStringLibrary.Conv_NameToString` (`self.Name`))))
  (`TimelineComponent.SetNewTime` (`self.Click`) 0.0)
  (`self.On Interact`)
  (return true))

(fn `UserConstructionScript`)