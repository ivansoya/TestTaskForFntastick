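; BP_Turtle is a "turtle" actor that travels to its assigned FinishPoint, where it spawns a heal-aura effect and destroys itself.
; It attaches a fire-storm particle and steam sound to its mesh on BeginPlay.
; ReadyToWork picks behavior by turtle number: one keeps a constant state, the others run a self-recalling delay loop that alternates CurrentState between base and alternate states.
; The controller reads CurrentState to decide its action.
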(event `self.ReceiveBeginPlay`
  (bind _mesh (`self.Mesh`))
  ;[1 1 1] Спавн эфекта и привязка звука к модели "черепашки"
  (`GameplayStatics.SpawnEmitterAttached` "/Game/FXVarietyPack/Particles/P_ky_fireStorm.P_ky_fireStorm" _mesh "None" (0.0 0.0 0.0) (struct) (0.5 0.5 0.05))
  (`GameplayStatics.SpawnSoundAttached` "/Game/StarterContent/Audio/Steam01.Steam01" _mesh "None" (0.0 0.0 0.0) (struct) "KeepRelativeOffset" true 1.0 1.0 0.0 null null))

(event `self.ReceiveActorBeginOverlap`
  (params (OtherActor :type "Actor Object Reference"))
  (bind _finishpoint (`self.FinishPoint`))
  ;[1 1 1] Проверка нужного гнезда для черепашки
  (bind _asbp_finish_point (cast `/Game/Blueprints/BP_FinishPoint` OtherActor))
  (`/Engine/EditorBlueprintResources/StandardMacros.IsValid` _finishpoint
    (:`Is Valid`
      (if (== _asbp_finish_point _finishpoint)
        ;[1 1 1] Спавн эффекта и удаление "черепашки"
        (`|SpawnActorFromClass` "/Game/FXVarietyPack/Blueprints/BP_ky_healAura.BP_ky_healAura_C" (`self.GetTransform` _finishpoint) "AlwaysSpawn" "OverrideRootScale" null "/Game/Sound/SLevelUp.SLevelUp" null)
        (`self.K2_DestroyActor`)))))

(event `ReadyToWork`
  ;[1 1 1] Меняет поведение "черепашки" в зависимости от ее номера
  (switch `int` (`self.NumberOfTurtle`)
    (:`1`
      (set `self.CurrentState` "NewEnumerator0"))
    (:`2`
      (`self.ChangeBehavior` "NewEnumerator1"))
    (:`3`
      (`self.ChangeBehavior` "NewEnumerator2"))))

(event `ChangeBehavior`
  (params (NewState :type "/Game/Blueprints/EStates Enum" :default "NewEnumerator0") (BaseState :type "/Game/Blueprints/EStates Enum" :default "NewEnumerator0"))
  ;[1 1 1] Поведенческий цикл, меняет состояние "черепашки", чтобы контроллер мог определить, что ему делать
  (`KismetSystemLibrary.Delay` 1.0)
  (set `self.CurrentState` NewState)
  (`KismetSystemLibrary.Delay` 0.5)
  (set `self.CurrentState` BaseState)
  (`self.ChangeBehavior` NewState BaseState))

(fn `UserConstructionScript`)